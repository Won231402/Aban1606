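; BP_MoveRect is an actor whose static mesh loops around a square path in its local X-Z plane.
; Tick switches on the MoveType enum and calls one of four direction functions with frame time scaled by Speed.
; Each function offsets the mesh's relative location and sets the next direction once it passes its edge, forming a simple state machine.
; The event graph also holds disconnected practice nodes for branch and switch logic that never run.
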(event EventBeginPlay)

(event EventTick
  (params (DeltaSeconds :type Float%20%28single-precision%29))
  (bind _speed (Variables|Default|Getspeed))
  (bind _returnvalue (* DeltaSeconds _speed))
  (switch Utilities|FlowControl|Switch|SwitchonEN_MoveType (Variables|Default|GetMoveType)
    (:NewEnumerator0
      (CallFunction|MoveRight _returnvalue))
    (:NewEnumerator1
      (CallFunction|MoveUp _returnvalue))
    (:NewEnumerator2
      (CallFunction|MoveLeft _returnvalue))
    (:NewEnumerator3
      (CallFunction|MoveDown _returnvalue))))

(fn ConstructionScript)

(fn MoveRight
  (params (DeltaLocation_X :type Float%20%28double-precision%29))
  (bind _staticmesh (Variables|Default|GetStaticMesh))
  (Transformation|AddRelativeLocation _staticmesh (Math|Vector|MakeVector DeltaLocation_X 0.0 0.0) false false)
  (if (>= (.x (Variables|/Script/Engine.SceneComponent|GetRelativeLocation _staticmesh)) 5e+01)
    (Variables|Default|SetMoveType "NewEnumerator1")))

(fn MoveUp
  (params (DeltaLocation_Z :type Float%20%28double-precision%29))
  (bind _staticmesh (Variables|Default|GetStaticMesh))
  (Transformation|AddRelativeLocation _staticmesh (Math|Vector|MakeVector 0.0 0.0 DeltaLocation_Z) false false)
  (if (>= (.z (Variables|/Script/Engine.SceneComponent|GetRelativeLocation _staticmesh)) 5e+01)
    (Variables|Default|SetMoveType "NewEnumerator2")))

(fn MoveLeft
  (params (A :type Float%20%28double-precision%29))
  (bind _staticmesh (Variables|Default|GetStaticMesh))
  (Transformation|AddRelativeLocation _staticmesh (Math|Vector|MakeVector (* A -1.0) 0.0 0.0) false false)
  (if (< (.x (Variables|/Script/Engine.SceneComponent|GetRelativeLocation _staticmesh)) 0.0)
    (Variables|Default|SetMoveType "NewEnumerator3")))

(fn MoveDown
  (params (A :type Float%20%28double-precision%29))
  (bind _staticmesh (Variables|Default|GetStaticMesh))
  (Transformation|AddRelativeLocation _staticmesh (Math|Vector|MakeVector 0.0 0.0 (* A -1.0)) false false)
  (if (< (.z (Variables|/Script/Engine.SceneComponent|GetRelativeLocation _staticmesh)) 0.0)
    (Variables|Default|SetMoveType "NewEnumerator0")))