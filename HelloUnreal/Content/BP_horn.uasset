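; BP_horn is a Blueprint with a Cone component that spins and bobs up and down continuously.
; Each Tick adds a fixed yaw rotation, which is not scaled by delta time, so spin speed follows frame rate.
; Vertical movement uses Speed times DeltaSeconds, with the IsMoveUp flag flipping direction at fixed relative-height limits.
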(event EventTick
  (params (DeltaSeconds :type Float%20%28single-precision%29))
  (bind _cone (Variables|Default|GetCone))
  (bind _cone_2 (Variables|Default|GetCone))
  ;[1 1 1] 회전
  (Transformation|AddRelativeRotation (Variables|Default|GetCone) (Math|Rotator|MakeRotator 0.0 0.0 1e+01) false false)
  (if (Variables|Default|GetisMoveUp)
    ;[1 1 1] 위로 이동
    (Transformation|AddRelativeLocation _cone_2 (Math|Vector|MakeVector 0.0 0.0 (* DeltaSeconds (Variables|Default|Getspeed))) false false)
    (if (>= (.z (Variables|/Script/Engine.SceneComponent|GetRelativeLocation _cone_2)) 2e+01)
      (Variables|Default|SetisMoveUp false))
    (else
      ;[1 1 1] 아래로 이동
      (Transformation|AddRelativeLocation _cone (Math|Vector|MakeVector 0.0 0.0 (* (* DeltaSeconds (Variables|Default|Getspeed)) -1.0)) false false)
      (if (<= (.z (Variables|/Script/Engine.SceneComponent|GetRelativeLocation _cone)) 0.0)
        (Variables|Default|SetisMoveUp true)))))

(fn ConstructionScript)