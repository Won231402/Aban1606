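; Collectible coin pickup that spins in place and respawns after being collected.
; A fast looping timer rotates the mesh, while overlap by the third-person character adds a coin to its PlayerState.
; Collection hides the mesh and disables its collision until a timer restores both a few seconds later.
; BeginPlay caches a tagged portal, but its overlap notification is disconnected, leaving that reference unused.
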(event OnComponentBeginOverlap(StaticMesh)
  (params (OverlappedComponent :type Primitive%20Component%20Object%20Reference) (OtherActor :type Actor%20Object%20Reference) (OtherComp :type Primitive%20Component%20Object%20Reference) (OtherBodyIndex :type Integer) (bFromSweep :type Boolean) (SweepResult :type Hit%20Result%20Structure%20%28by%20ref%29))
  (bind _staticmesh (Variables|Default|GetStaticMesh))
  (bind _asbp_third_person_character (Utilities|Casting|CastToBP_ThirdPersonCharacter OtherActor))
  (bind _asbp_player_state (Utilities|Casting|CastToBP_PlayerState (Variables|/Script/Engine.Pawn|GetPlayerState _asbp_third_person_character)))
  (Default|AddCoin _asbp_player_state)
  (Rendering|SetVisibility _staticmesh false false)
  (Collision|SetCollisionEnabled _staticmesh "NoCollision")
  (Utilities|Time|SetTimerbyFunctionName 0 "ShowCoin" 5.0))

(event EventBeginPlay
  (Utilities|Time|SetTimerbyFunctionName 0 "UpdateRotation" 0.003 true)
  (bind _outactors (Actor|GetAllActorsOfClasswithTag "/Game/CoinGame/BP_Portal00.BP_Portal00_C" (Variables|Default|GetPortalTag)))
  (for _array_element _outactors
    (Variables|Default|SetPotal _array_element)))

(fn ConstructionScript)

(fn UpdateRotation
  (Transformation|AddRelativeRotation (Variables|Default|GetStaticMesh) "0.000000,1.000000,0.000000" false false))

(fn ShowCoin
  (bind _staticmesh (Variables|Default|GetStaticMesh))
  (Rendering|SetVisibility _staticmesh true false)
  (Collision|SetCollisionEnabled _staticmesh "QueryAndPhysics"))