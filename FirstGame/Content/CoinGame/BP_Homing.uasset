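; Homing projectile in the coin game that chases the first player's character and explodes on overlap.
; BeginPlay sets the target; Tick moves it along its Arrow by a frame-rate-dependent step and eases its rotation toward the target for curved pursuit.
; Sphere overlap with a BP_ThirdPersonCharacter adds damage through BP_PlayerState and triggers ragdoll.
; Any overlap then spawns an explosion and destroys the projectile.
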(event OnComponentBeginOverlap(Sphere)
  (params (OverlappedComponent :type Primitive%20Component%20Object%20Reference) (OtherActor :type Actor%20Object%20Reference) (OtherComp :type Primitive%20Component%20Object%20Reference) (OtherBodyIndex :type Integer) (bFromSweep :type Boolean) (SweepResult :type Hit%20Result%20Structure%20%28by%20ref%29))
  (CallFunction|EventHitCharacter OtherActor)
  (CallFunction|DestroyHoming))

(event EventTick
  (params (DeltaSeconds :type Float%20%28single-precision%29))
  (Utilities|IsValid (Variables|Default|GetHomingTarget)
    (:Is%20Valid
      (Transformation|AddActorWorldOffset (* (Math|Vector|GetForwardVector (Variables|Default|GetArrow)) 5.0))
      (Transformation|SetActorRotation (Math|Interpolation|RInterpTo (Transformation|GetActorRotation) (Math|Rotator|FindLookatRotation (Transformation|GetActorLocation) (Transformation|GetActorLocation (Variables|Default|GetHomingTarget))) DeltaSeconds 2.0)))))

(event EventBeginPlay
  (Variables|Default|SetHomingTarget (Game|GetPlayerCharacter 0)))

(fn ConstructionScript)

(fn DestroyHoming
  (Effects|SpawnEmitteratLocation "/Game/StarterContent/Particles/P_Explosion.P_Explosion" (Transformation|GetActorLocation) (Transformation|GetActorRotation))
  (Actor|DestroyActor))

(fn EventHitCharacter
  (params (Actor :type Actor%20Object%20Reference))
  (bind _asbp_third_person_character (Utilities|Casting|CastToBP_ThirdPersonCharacter Actor))
  (bind _asbp_player_state (Utilities|Casting|CastToBP_PlayerState (Variables|/Script/Engine.Pawn|GetPlayerState _asbp_third_person_character)))
  (Default|AddDamage _asbp_player_state 1e+01)
  (Default|DoRagdoll _asbp_third_person_character))