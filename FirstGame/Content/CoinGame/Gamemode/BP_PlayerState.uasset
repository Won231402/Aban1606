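; BP_PlayerState is the player state for the coin game, keeping the player's Coin and SilverItem counts.
; AddCoin and AddSilverItem each increment their counter by one, then cast the first player controller's HUD to BP_Hud and push the new total to its matching text setter.
; The HUD lookup always uses player index 0, and the event graph and construction script hold no logic.
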(event EventBeginPlay)

(event EventTick
  (params (DeltaSeconds :type Float%20%28single-precision%29)))

(fn ConstructionScript)

(fn AddCoin
  (bind _output_get (Variables|Default|SetCoin (+ (Variables|Default|GetCoin) 1)))
  (bind _asbp_hud (Utilities|Casting|CastToBP_Hud (HUD|GetHUD (Game|GetPlayerController 0))))
  (Default|SetCoinText _asbp_hud _output_get))

(fn AddSilverItem
  (bind _output_get (Variables|Default|SetSilverItem (+ (Variables|Default|GetSilverItem) 1)))
  (bind _asbp_hud (Utilities|Casting|CastToBP_Hud (HUD|GetHUD (Game|GetPlayerController 0))))
  (Default|SetSilverItemText _asbp_hud _output_get))