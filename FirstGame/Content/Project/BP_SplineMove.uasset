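; BP_SplineMove is a Blueprint that moves a Cube back and forth along a Spline.
; EventPlay runs a timeline forward or in reverse based on IsRight, and each update scales its track value by the spline length to set the Cube's world location.
; When the timeline finishes, IsRight flips and the branch runs again for continuous ping-pong motion, while EventStop halts the timeline.
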(event EventBeginPlay)

(event EventEventPlay
  (bind _spline (Variables|Default|GetSpline))
  (if (Variables|Default|GetisRight) :!label _label
    (bind _새_트랙_0 (Timeline|타임라인 Play)
      (:Update
        (Transformation|SetWorldLocation (Variables|Default|GetCube) (Spline|GetLocationatDistanceAlongSpline _spline (* _새_트랙_0 (Spline|GetSplineLength _spline)) "World") false false))
      (:Finished
        (Variables|Default|SetisRight (not (Variables|Default|GetisRight)))
        (goto _label)))
    (else
      (Timeline|타임라인 Reverse))))

(event EventEventStop
  (bind _spline (Variables|Default|GetSpline))
  (bind _새_트랙_0 (Timeline|타임라인 Stop)
    (:Update
      (Transformation|SetWorldLocation (Variables|Default|GetCube) (Spline|GetLocationatDistanceAlongSpline _spline (* _새_트랙_0 (Spline|GetSplineLength _spline)) "World") false false))
    (:Finished
      (Variables|Default|SetisRight (not (Variables|Default|GetisRight)))
      (if (Variables|Default|GetisRight)
        (Timeline|타임라인 Play)
        (else
          (Timeline|타임라인 Reverse))))))

(fn ConstructionScript)