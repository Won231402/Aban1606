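; BP_MoveLeftRight is an actor whose static mesh shuttles back and forth along its relative X axis.
; Tick moves the mesh a fixed step per frame, not scaled by delta time, and flips the Moveleftright flag when it reaches either end of a hard-coded range.
; EventPlay and EventStop start and pause the motion by setting the Moveplay flag.
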(event EventTick
  (params (DeltaSeconds :type Float%20%28single-precision%29))
  (bind _staticmesh (Variables|Default|GetStaticMesh))
  (bind _staticmesh_2 (Variables|Default|GetStaticMesh))
  (if (Variables|Default|Getmoveplay)
    (if (Variables|Default|Getmoveleftright)
      (Transformation|AddRelativeLocation _staticmesh_2 "10.000000,0.000000,0.000000" false false)
      (if (>= (.x (Variables|/Script/Engine.SceneComponent|GetRelativeLocation _staticmesh_2)) 3e+02)
        (Variables|Default|Setmoveleftright false))
      (else
        (Transformation|AddRelativeLocation _staticmesh "-10.000000,0.000000,0.000000" false false)
        (if (< (.x (Variables|/Script/Engine.SceneComponent|GetRelativeLocation _staticmesh)) 0.0)
          (Variables|Default|Setmoveleftright true))))))

(event EventEventPlay
  (Variables|Default|Setmoveplay true))

(event EventEventStop
  (Variables|Default|Setmoveplay false))

(fn ConstructionScript)