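; BP_SplineMove03 is a moving hazard whose cube travels along a spline and ragdolls the third-person character when it registers a hit.
; A timeline scales its track value by spline length to set the cube's world location without sweeping.
; EventPlay starts the timeline, which flips IsRight on finishing to alternate Play and Reverse in a ping-pong loop.
; EventStop halts it.
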(event OnComponentHit(Cube)
  (params (HitComponent :type Primitive%20Component%20Object%20Reference) (OtherActor :type Actor%20Object%20Reference) (OtherComp :type Primitive%20Component%20Object%20Reference) (NormalImpulse :type Vector :default "0, 0, 0") (Hit :type Hit%20Result%20Structure%20%28by%20ref%29))
  (bind _asbp_third_person_character (Utilities|Casting|CastToBP_ThirdPersonCharacter OtherActor))
  (Default|DoRagdoll _asbp_third_person_character))

(event EventEventPlay
  (bind _spline (Variables|Default|GetSpline))
  (if (Variables|Default|GetisRight) :!label _label
    (bind _새_트랙_0 (Timeline|타임라인 Play)
      (:Update
        (Transformation|SetWorldLocation (Variables|Default|GetCube) (Spline|GetLocationatDistanceAlongSpline _spline (* _새_트랙_0 (Spline|GetSplineLength _spline)) "World") false false))
      (:Finished
        (Variables|Default|SetisRight (not (Variables|Default|GetisRight)))
        (goto _label)))
    (else
      (Timeline|타임라인 Reverse))))

(event EventEventStop
  (bind _spline (Variables|Default|GetSpline))
  (bind _새_트랙_0 (Timeline|타임라인 Stop)
    (:Update
      (Transformation|SetWorldLocation (Variables|Default|GetCube) (Spline|GetLocationatDistanceAlongSpline _spline (* _새_트랙_0 (Spline|GetSplineLength _spline)) "World") false false))
    (:Finished
      (Variables|Default|SetisRight (not (Variables|Default|GetisRight)))
      (if (Variables|Default|GetisRight)
        (Timeline|타임라인 Play)
        (else
          (Timeline|타임라인 Reverse))))))

(fn ConstructionScript)