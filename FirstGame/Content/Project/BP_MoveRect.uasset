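; Actor that moves its static mesh around a rectangular loop in the local XZ plane while play is enabled.
; Tick runs a Move enum state machine (Right, Up, Left, Down) that offsets the mesh by a fixed, frame-rate-dependent step and switches direction when its relative location crosses the bounds.
; EventPlay and EventStop toggle the Isplay flag to start or pause the motion.
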(event EventTick
  (params (DeltaSeconds :type Float%20%28single-precision%29))
  (bind _staticmesh (Variables|Default|GetStaticMesh))
  (bind _staticmesh_2 (Variables|Default|GetStaticMesh))
  (bind _staticmesh_3 (Variables|Default|GetStaticMesh))
  (bind _staticmesh_4 (Variables|Default|GetStaticMesh))
  (if (Variables|Default|Getisplay)
    (switch Utilities|FlowControl|Switch|SwitchonEN_MoveActor (Variables|Default|Getmove)
      (:NewEnumerator0
        (Transformation|AddRelativeLocation _staticmesh_2 "10.000000,0.000000,0.000000" false false)
        (if (>= (.x (Variables|/Script/Engine.SceneComponent|GetRelativeLocation _staticmesh_2)) 2e+02)
          (Variables|Default|Setmove "NewEnumerator1")))
      (:NewEnumerator1
        (Transformation|AddRelativeLocation _staticmesh_3 "0.000000,0.000000,10.000000" false false)
        (if (>= (.z (Variables|/Script/Engine.SceneComponent|GetRelativeLocation _staticmesh_3)) 2e+02)
          (Variables|Default|Setmove "NewEnumerator2")))
      (:NewEnumerator2
        (Transformation|AddRelativeLocation _staticmesh_4 "-10.000000,0.000000,0.000000" false false)
        (if (< (.x (Variables|/Script/Engine.SceneComponent|GetRelativeLocation _staticmesh_4)) 0.0)
          (Variables|Default|Setmove "NewEnumerator3")))
      (:NewEnumerator3
        (Transformation|AddRelativeLocation _staticmesh "0.000000,0.000000,-10.000000" false false)
        (if (< (.z (Variables|/Script/Engine.SceneComponent|GetRelativeLocation _staticmesh)) 0.0)
          (Variables|Default|Setmove "NewEnumerator0"))))))

(event EventEventPlay
  (Variables|Default|Setisplay true))

(event EventEventStop
  (Variables|Default|Setisplay false))

(fn ConstructionScript)