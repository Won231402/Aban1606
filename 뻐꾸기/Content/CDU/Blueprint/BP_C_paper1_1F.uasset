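; BP_C_paper1_1F is a paper pickup that stays invisible and non-collidable until no BP_PaperPiece actors remain in the world.
; Tick polls for remaining pieces with GetAllActorsOfClass every frame, then enables the mesh's visibility and collision once none are found.
; When a BP_ThirdPersonCharacter with a BP_PlayerState overlaps the mesh, it hides the actor and calls StairActivate on its StairActivate reference.
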(event OnComponentBeginOverlap(StaticMesh)
  (params (OverlappedComponent :type Primitive%20Component%20Object%20Reference) (OtherActor :type Actor%20Object%20Reference) (OtherComp :type Primitive%20Component%20Object%20Reference) (OtherBodyIndex :type Integer) (bFromSweep :type Boolean) (SweepResult :type Hit%20Result%20Structure%20%28by%20ref%29))
  (bind _asbp_third_person_character (Utilities|Casting|CastToBP_ThirdPersonCharacter OtherActor))
  (Utilities|Casting|CastToBP_PlayerState (Variables|/Script/Engine.Pawn|GetPlayerState _asbp_third_person_character))
  (Rendering|SetActorHiddenInGame true)
  (Default|StairActivate (Variables|Default|GetStairActivate)))

(event EventBeginPlay
  (CallFunction|ShowCPaper false))

(event EventTick
  (params (DeltaSeconds :type Float%20%28single-precision%29))
  (CallFunction|CheckShowCPaper))

(fn ConstructionScript)

(fn IsGetAllPaper
  (bind _outactors (Actor|GetAllActorsOfClass "/Game/CDU/Blueprint/BP_PaperPiece.BP_PaperPiece_C"))
  (for _array_element _outactors
    (return false))
  (return true))

(fn CheckShowCPaper
  (bind _isgetall (CallFunction|IsGetAllPaper))
  (if _isgetall
    (CallFunction|ShowCPaper true)))

(fn ShowCPaper
  (params (BeShow :type Boolean))
  (bind _staticmesh (Variables|Default|GetStaticMesh))
  (if BeShow
    (Rendering|SetVisibility _staticmesh true false)
    (Collision|SetCollisionEnabled _staticmesh "QueryAndPhysics")
    (else
      (Rendering|SetVisibility _staticmesh false false)
      (Collision|SetCollisionEnabled 0 "NoCollision"))))