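; BP_Bullet is a physics-driven projectile that damages and ragdolls third-person player characters on impact.
; On BeginPlay it launches its Sphere with a large forward impulse and destroys itself after two seconds.
; A Sphere hit on a BP_ThirdPersonCharacter adds damage through its BP_PlayerState and triggers ragdoll.
; Any hit spawns an explosion sound and sparks effect, then destroys the bullet.
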(event OnComponentHit(Sphere)
  (params (HitComponent :type Primitive%20Component%20Object%20Reference) (OtherActor :type Actor%20Object%20Reference) (OtherComp :type Primitive%20Component%20Object%20Reference) (NormalImpulse :type Vector :default "0, 0, 0") (Hit :type Hit%20Result%20Structure%20%28by%20ref%29))
  (CallFunction|EventHitCharacter OtherActor)
  (CallFunction|DestroyBullet))

(event EventBeginPlay
  (Physics|AddImpulse (Variables|Default|GetSphere) (* (Transformation|GetActorForwardVector) 5e+06) "None" false)
  (Utilities|FlowControl|Delay 2.0)
  (Actor|DestroyActor))

(fn ConstructionScript)

(fn DestroyBullet
  (Audio|SpawnSoundatLocation "/Game/StarterContent/Audio/Explosion01.Explosion01" (Transformation|GetActorLocation) "0, 0, 0" 1.0 1.0 0.0 0 0)
  (Effects|SpawnEmitteratLocation "/Game/StarterContent/Particles/P_Sparks.P_Sparks" (Transformation|GetActorLocation) (Transformation|GetActorRotation) "0.500000,0.500000,0.500000")
  (Actor|DestroyActor))

(fn EventHitCharacter
  (params (actor :type Actor%20Object%20Reference))
  (bind _asbp_third_person_character (Utilities|Casting|CastToBP_ThirdPersonCharacter actor))
  (bind _asbp_player_state (Utilities|Casting|CastToBP_PlayerState (Variables|/Script/Engine.Pawn|GetPlayerState _asbp_third_person_character)))
  (Default|AddDamage _asbp_player_state 5.0)
  (Default|DoRagdoll _asbp_third_person_character))