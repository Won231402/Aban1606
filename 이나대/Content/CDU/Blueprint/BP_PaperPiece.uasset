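; BP_PaperPiece is a collectible paper pickup that spins in place until a player collects it.
; A fast looping timer started at BeginPlay rotates the static mesh in small steps, without using Tick.
; When a BP_ThirdPersonCharacter overlaps the mesh, it calls AddPaper on that character's BP_PlayerState and destroys itself.
; An unconnected branch that would hide the mesh and disable its collision never runs.
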(event OnComponentBeginOverlap(StaticMesh)
  (params (OverlappedComponent :type Primitive%20Component%20Object%20Reference) (OtherActor :type Actor%20Object%20Reference) (OtherComp :type Primitive%20Component%20Object%20Reference) (OtherBodyIndex :type Integer) (bFromSweep :type Boolean) (SweepResult :type Hit%20Result%20Structure%20%28by%20ref%29))
  (bind _asbp_third_person_character (Utilities|Casting|CastToBP_ThirdPersonCharacter OtherActor))
  (bind _asbp_player_state (Utilities|Casting|CastToBP_PlayerState (Variables|/Script/Engine.Pawn|GetPlayerState _asbp_third_person_character)))
  (Default|AddPaper _asbp_player_state)
  (Actor|DestroyActor))

(event EventBeginPlay
  (Utilities|Time|SetTimerbyFunctionName 0 "Update Rotation" 0.01 true))

(event Collision|EventActorBeginOverlap
  (params (OtherActor :type Actor%20Object%20Reference)))

(event EventTick
  (params (DeltaSeconds :type Float%20%28single-precision%29)))

(fn ConstructionScript)

(fn UpdateRotation
  (Transformation|AddRelativeRotation (Variables|Default|GetStaticMesh) "0.000000,1.000000,0.000000" false false))