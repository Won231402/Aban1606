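; BP_MoveDoor_2F is a door that opens when enough pressure buttons are active.
; ButtonActivated and ButtonDeactivated raise or lower a counter, then play or reverse the DoorActivation timeline depending on whether it meets PressureButtonNeeds.
; The timeline drives the door mesh's relative yaw, so the door swings rather than slides.
; An older variant that moves the door vertically remains as disconnected, unused nodes.
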(event Custom|ButtonActivated
  (Math|Integer|IncrementInt (Variables|Default|GetPressureButtonActivate)
    (:%20%20
      (if (>= (Variables|Default|GetPressureButtonActivate) (Variables|Default|GetPressureButtonNeeds))
        (bind _doorposition (Timeline|DoorActivation Play)
          (:Update
            (Transformation|SetRelativeRotation (Variables|Default|GetMoveDoor) (Math|Rotator|MakeRotator 0.0 0.0 _doorposition) false false)))
        (else
          (Timeline|DoorActivation Reverse))))))

(event Custom|ButtonDeactivated
  (Math|Integer|DecrementInt (Variables|Default|GetPressureButtonActivate)
    (:%20%20
      (if (>= (Variables|Default|GetPressureButtonActivate) (Variables|Default|GetPressureButtonNeeds))
        (bind _doorposition (Timeline|DoorActivation Play)
          (:Update
            (Transformation|SetRelativeRotation (Variables|Default|GetMoveDoor) (Math|Rotator|MakeRotator 0.0 0.0 _doorposition) false false)))
        (else
          (Timeline|DoorActivation Reverse))))))

(event EventBeginPlay)

(event Collision|EventActorBeginOverlap
  (params (OtherActor :type Actor%20Object%20Reference)))

(event EventTick
  (params (DeltaSeconds :type Float%20%28single-precision%29)))

(fn ConstructionScript)