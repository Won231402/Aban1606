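; BP_MoveLRBox is an actor whose Cube slides back and forth along its local X axis.
; Each Tick offsets the Cube's relative location by Speed scaled by delta time, in the direction set by the MoveRight flag.
; The flag flips once the Cube reaches or passes either hardcoded bound, 0 or 1500, with no clamping of the overshoot.
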(event EventTick
  (params (DeltaSeconds :type Float%20%28single-precision%29))
  (bind _cube (Variables|Default|GetCube))
  (bind _speed (Variables|Default|GetSpeed))
  (bind _cube_2 (Variables|Default|GetCube))
  (bind _returnvalue (* DeltaSeconds _speed))
  (if (Variables|Default|GetMoveRight)
    (Transformation|AddRelativeLocation _cube_2 (Math|Vector|MakeVector _returnvalue 0.0 0.0) false false)
    (if (>= (.x (Variables|/Script/Engine.SceneComponent|GetRelativeLocation _cube_2)) 1.5e+03)
      (Variables|Default|SetMoveRight false))
    (else
      (Transformation|AddRelativeLocation _cube (Math|Vector|MakeVector (* _returnvalue -1.0) 0.0 0.0) false false)
      (if (<= (.x (Variables|/Script/Engine.SceneComponent|GetRelativeLocation _cube)) 0.0)
        (Variables|Default|SetMoveRight true)))))

(fn ConstructionScript)