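; BP_HelloActor is a practice actor that slides its Sphere component back and forth along relative X.
; On BeginPlay it prints its display name in red, runs a small addition and an empty loop, then prints "complete".
; Tick moves the sphere by DeltaSeconds times Speed, flipping IsMoveRight at the range limits.
; Several disconnected experiments with printing, loops, transforms, math and string append remain unexecuted.
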(event EventBeginPlay
  (Development|PrintString (Utilities|GetDisplayName self) true true "(R=1.000000,G=0.000000,B=0.000000,A=1.000000)" 6e+01)
  (Variables|Default|Setx축의%20값 (+ 1.0 1.0))
  (for _index (range 0 5)
    _)
  (Development|PrintString "complete" true true "(R=0.000000,G=0.660000,B=1.000000,A=1.000000)" 6e+01))

(event EventTick
  (params (DeltaSeconds :type Float%20%28single-precision%29))
  (bind _sphere (Variables|Default|GetSphere))
  (bind _sphere_2 (Variables|Default|GetSphere))
  (if (Variables|Default|GetisMoveRight)
    ;[1 0.2396 0.2396] 오른쪽으로 이동
    (Transformation|AddRelativeLocation _sphere (Math|Vector|MakeVector (* DeltaSeconds (Variables|Default|Getspeed)) 0.0 0.0) false false)
    (if (>= (.x (Variables|/Script/Engine.SceneComponent|GetRelativeLocation _sphere)) 5.0)
      (Variables|Default|SetisMoveRight false))
    (else
      ;[0.2622 0.2689 1] 왼쪽으로 이동
      (Transformation|AddRelativeLocation _sphere_2 (Math|Vector|MakeVector (* (* DeltaSeconds (Variables|Default|Getspeed)) -1.0) 0.0 0.0) false false)
      (if (<= (.x (Variables|/Script/Engine.SceneComponent|GetRelativeLocation _sphere_2)) 0.0)
        (Variables|Default|SetisMoveRight true)))))

(fn ConstructionScript)